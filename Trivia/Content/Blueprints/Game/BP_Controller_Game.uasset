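; Player controller that opens the lobby UI and triggers player list updates as players arrive and leave.
; On BeginPlay it shows the mouse cursor, sets UI-only input and adds a W_UI_Lobby widget to the viewport.
; BeginPlay and Destroyed both call ServerUpdatePlayerList, which casts the game state to BP_GameState_Game and calls CallOnPlayerUpdate.
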(event `self.ReceiveBeginPlay`
  (set `self.bShowMouseCursor` true)
  (`WidgetBlueprintLibrary.SetInputMode_UIOnlyEx` (`GameplayStatics.GetPlayerController` 0) null)
  (bind _returnvalue (`|CreateWidget` "/Game/Blueprints/Game/UI/W_UI_Lobby.W_UI_Lobby_C" (`GameplayStatics.GetPlayerController` 0)))
  (`UserWidget.AddToViewport` _returnvalue 0)
  (`self.ServerUpdatePlayerList`))

(event `ServerUpdatePlayerList`
  (bind _asbp_game_state_game (cast `/Game/Blueprints/Game/BP_GameState_Game` (`GameplayStatics.GetGameState`)))
  (`/Game/Blueprints/Game/BP_GameState_Game.CallOnPlayerUpdate` _asbp_game_state_game))

(event `self.ReceiveDestroyed`
  (`self.ServerUpdatePlayerList`))

(fn `UserConstructionScript`)