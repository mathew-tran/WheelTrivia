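; Game state for a multiplayer, turn-based hangman-style phrase game with shared points and game over at five failed guesses.
; SetupGame shuffles DT_Phrases rows and picks a random starting player; each round builds masked and complete letter arrays from the answer.
; TryLetter reveals matches, updates score and streak multiplier, passes the turn by player name, and starts the next round when solved.
; OnRep functions relay turn, score and failure changes through dispatchers.
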(event `CallOnPlayerUpdate`
  (`self.OnPlayerUpdate`))

(event `SetupGame`
  (bind _outrownames (`DataTableFunctionLibrary.GetDataTableRowNames` "/Game/Blueprints/Game/Data/DT_Phrases.DT_Phrases"))
  (bind _output_get (set `self.Questions` _outrownames))
  (`KismetArrayLibrary.Array_Shuffle` _output_get)
  (`self.Define Start Player Turn`)
  (`self.StartRound`))

(event `StartRound`
  (`KismetArrayLibrary.Array_Clear` (`self.DisabledLetters`))
  (bind _returnvalue (`|GetDataTableRow` "/Game/Blueprints/Game/Data/DT_Phrases.DT_Phrases" (`|GetArrayItem` (`self.Questions`) (`self.Index`)))
    (:`then`
      (bind (_prompt _answer) (break `/Game/Blueprints/Game/Data/DS_Phrases` _returnvalue))
      (set `self.Prompt` _prompt)
      (set `self.Answer` (`KismetStringLibrary.ToUpper` _answer))
      (`self.MakeAnswerHidden`)
      (set `self.AnswerBuilder` (`self.AnswerBuilder`))
      (set `self.AnswerBuilderComplete` (`self.AnswerBuilderComplete`))
      (set `self.Index` (+ (`self.Index`) 1)))))

(event `UpdatePoints`
  (params (Points :type Integer)))

(event `Define Start Player Turn`
  (set `self.CurrentPlayersTurn` (`PlayerState.GetPlayerName` (`KismetArrayLibrary.Array_Random` (`self.PlayerArray`)))))

(event `AddPoints`
  (params (PointAmount :type Integer))
  (bind _output_get (set `self.PointsGained` (* PointAmount (`self.PointsMultiplier`))))
  (set `self.Points` (+ _output_get (`self.Points`))))

(event `UpdateMultiplier`
  (params (bIsIncreased :type Boolean))
  (if bIsIncreased
    (set `self.PointsMultiplier` (+ (`self.PointsMultiplier`) 0.1))
    (else
      (set `self.PointsMultiplier` 1.0))))

(event `TryLetter`
  (params (Letter :type String))
  (set `self.HasAddedLetter` false)
  (for (_array_element _array_index) (`self.AnswerBuilderComplete`)
    (if (`KismetStringLibrary.EqualEqual_StrStr` _array_element Letter)
      (`KismetArrayLibrary.Array_Set` (`self.AnswerBuilder`) _array_index Letter)
      (set `self.HasAddedLetter` true)
      (`self.AddPoints` 10)))
  (`KismetArrayLibrary.Array_Add` (`self.DisabledLetters`) Letter)
  (set `self.DisabledLetters` (`self.DisabledLetters`))
  (set `self.AnswerBuilder` (`self.AnswerBuilder`))
  (`self.CyclePlayerTurn`)
  (`self.UpdateMultiplier` (`self.HasAddedLetter`))
  (`self.DetermineEndRound`))

(event `CyclePlayerTurn`
  (for _array_element (`self.PlayerArray`)
    (bind _returnvalue (`PlayerState.GetPlayerName` _array_element))
    (if (`KismetStringLibrary.NotEqual_StrStr` _returnvalue (`self.CurrentPlayersTurn`))
      (bind _output_get (set `self.CurrentPlayersTurn` _returnvalue))
      (`KismetSystemLibrary.PrintString` _output_get)
      (break))))

(event `DetermineEndRound`
  (`self.HasFailedAttempt` (not (`self.HasAddedLetter`)))
  (if (`KismetArrayLibrary.Array_Identical` (`self.AnswerBuilderComplete`) (`self.AnswerBuilder`))
    (`self.StartRound`)
    (`KismetSystemLibrary.Delay` 0.3)
    (`self.AddPoints` 200)))

(event `HasFailedAttempt`
  (params (bHasFailed :type Boolean))
  (if bHasFailed
    (set `self.FailedAttempts` (+ (`self.FailedAttempts`) 1))))

(fn `GetAnswerBuilder`
  (returns (NewParam :type String))
  (locals (AnswerBuilderString :type String))
  (for _array_element (`self.AnswerBuilder`)
    (set `local.AnswerBuilderString` (`KismetStringLibrary.Concat_StrStr` (`local.AnswerBuilderString`) _array_element)))
  (return (`local.AnswerBuilderString`)))

(fn `IsGameOver`
  (returns (bIsGameOver :type Boolean))
  (return (== (`self.FailedAttempts`) 5)))

(fn `IsPlayersTurn`
  (params (PlayerState :type "PlayerState Object Reference"))
  (returns (IsPlayersTurn :type Boolean))
  (bind _currentplayersturn (`self.CurrentPlayersTurn`))
  (`KismetSystemLibrary.PrintString` _currentplayersturn)
  (return (`KismetStringLibrary.EqualEqual_StrStr` (`PlayerState.GetPlayerName` PlayerState) _currentplayersturn)))

(fn `MakeAnswerHidden`
  (bind _array (`|MakeArray` ""))
  (set `self.AnswerBuilderComplete` _array)
  (set `self.AnswerBuilder` _array)
  (for _index (range (`KismetStringLibrary.Len` (`self.Answer`)))
    (bind _returnvalue (`KismetStringLibrary.GetSubstring` (`self.Answer`) _index))
    (if (`KismetStringLibrary.EqualEqual_StrStr` _returnvalue " ")
      (`KismetArrayLibrary.Array_Add` (`self.AnswerBuilder`) "    ")
      (`KismetArrayLibrary.Array_Add` (`self.AnswerBuilderComplete`) "    ")
      (else
        (`KismetArrayLibrary.Array_Add` (`self.AnswerBuilder`) "_ ")
        (`KismetArrayLibrary.Array_Add` (`self.AnswerBuilderComplete`) _returnvalue)))))

(fn `OnRep_Answer`)

(fn `OnRep_AnswerBuilder`)

(fn `OnRep_CurrentPlayersTurn`
  (`self.OnTurnUpdate`))

(fn `OnRep_FailedAttempts`
  (`self.OnFailedAttemptsUpdate` (`self.FailedAttempts`)))

(fn `OnRep_Index`
  (`self.OnTurnUpdate`)
  (`self.OnStartGame`))

(fn `OnRep_Points`
  (`self.OnPointsUpdate` (`self.Points`)))

(fn `OnRep_PointsGained`
  (`self.OnPointsGained` (`self.PointsGained`)))

(fn `OnRep_Prompt`)

(fn `UserConstructionScript`)